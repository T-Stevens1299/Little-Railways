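; Victorian variant of the Bowsider railway carriage, built from child-actor bogies and couplings.
; On BeginPlay it gets each Bowsider bogie's root static mesh and passes it to the coupling at the same end through SetVehicleBodyMessage.
; This makes each bogie's mesh, rather than the carriage itself, the vehicle body its coupling receives.
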(event EventBeginPlay
  (CallFunction|SetCoupling1)
  (CallFunction|SetCoupling2))

(fn ConstructionScript)

(fn SetCoupling1
  (bind _asbp_bowsider_bogie (Utilities|Casting|CastToBP_BowsiderBogie (Variables|/Script/Engine.ChildActorComponent|GetChildActor (Variables|Default|GetBogie1))))
  (bind _asstatic_mesh_component (Utilities|Casting|CastToStaticMeshComponent (Variables|/Script/Engine.Actor|GetRootComponent _asbp_bowsider_bogie)))
  (Class|BPICoupling|SetVehicleBody(Message) (Variables|/Script/Engine.ChildActorComponent|GetChildActor (Variables|Default|GetCoupling1)) _asstatic_mesh_component))

(fn SetCoupling2
  (bind _asbp_bowsider_bogie (Utilities|Casting|CastToBP_BowsiderBogie (Variables|/Script/Engine.ChildActorComponent|GetChildActor (Variables|Default|GetBogie2))))
  (bind _asstatic_mesh_component (Utilities|Casting|CastToStaticMeshComponent (Variables|/Script/Engine.Actor|GetRootComponent _asbp_bowsider_bogie)))
  (Class|BPICoupling|SetVehicleBody(Message) (Variables|/Script/Engine.ChildActorComponent|GetChildActor (Variables|Default|GetCoupling2)) _asstatic_mesh_component))