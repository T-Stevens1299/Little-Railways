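; Game instance for Little Railways that saves, loads and deletes the game in one hardcoded slot.
; SaveData gathers locomotives with tender fuel and water, wagons, carriages with passengers, player possession or transform, and progression into BP_SaveGameObject.
; Rolling stock is stored as parallel arrays, appended on each save without clearing here.
; LoadGame only caches the save object and sets LoadingGame, with no restoration in this file.
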(event Custom|SaveGame
  (bind _returnvalue (SaveGame|DoesSaveGameExist "Test"))
  (if _returnvalue
    (CallFunction|SaveData)
    (bind _returnvalue_2 (SaveGame|SaveGametoSlot (Variables|Default|GetSaveGameObject) "Test"))
    (Development|PrintString (Utilities|String|Append "Game Saved:" (Utilities|String|ToString(Boolean) _returnvalue_2)))
    (else
      (bind _returnvalue_3 (SaveGame|CreateSaveGameObject "/Game/Blueprints/SaveSystem/BP_SaveGameObject.BP_SaveGameObject_C"))
      (Variables|Default|SetSaveGameObject _returnvalue_3)
      (CallFunction|SaveData)
      (bind _returnvalue_4 (SaveGame|SaveGametoSlot (Variables|Default|GetSaveGameObject) "Test"))
      (Development|PrintString (Utilities|String|Append "Game Saved:" (Utilities|String|ToString(Boolean) _returnvalue_4))))))

(event Custom|LoadGame
  (bind _returnvalue (SaveGame|DoesSaveGameExist "Test"))
  (if _returnvalue
    (bind _returnvalue_2 (SaveGame|LoadGamefromSlot "Test"))
    (bind _asbp_save_game_object (Utilities|Casting|CastToBP_SaveGameObject _returnvalue_2))
    (Variables|Default|SetSaveGameObject _asbp_save_game_object)
    (Variables|Default|SetLoadingGame true)))

(event Custom|NewGame
  (SaveGame|DeleteGameinSlot "Test"))

(fn SaveLocos
  (bind _locodata (Variables|Default|GetLocoData))
  (bind _outactors (Actor|GetAllActorsOfClass "/Script/LittleRailways.LocoController"))
  (for _array_element _outactors
    (Utilities|Array|Add (.locotypeid _locodata) (Variables|/Script/LittleRailways.LocoController|GettypeID _array_element))
    (bind _aslocomotive_tender (Utilities|Casting|CastToLocomotiveTender (Variables|/Script/Engine.ChildActorComponent|GetChildActor (Variables|/Script/LittleRailways.LocoController|GetTenderMesh _array_element))))
    (Utilities|Array|Add (.curfuelamount _locodata) (Variables|/Script/LittleRailways.LocomotiveTender|GetcurFuelAmount _aslocomotive_tender))
    (Utilities|Array|Add (.curwateramount _locodata) (Variables|/Script/LittleRailways.LocomotiveTender|GetcurWaterAmount _aslocomotive_tender))
    (Utilities|Array|Add (.spawntransform _locodata) (Transformation|GetActorTransform _array_element))
    (Development|PrintString (Utilities|String|ToString(Transform) (Transformation|GetActorTransform _array_element)) true true "(R=1.000000,G=0.000000,B=0.028711,A=1.000000)" 1e+01)))

(fn SaveWagons
  (bind _wagondata (Variables|Default|GetWagonData))
  (bind _outactors (Actor|GetAllActorsOfClass "/Script/LittleRailways.TestWagon"))
  (for _array_element _outactors
    (Utilities|Array|Add (.wagonclassid _wagondata) (Variables|/Script/LittleRailways.TestWagon|GettypeID _array_element))
    (Utilities|Array|Add (.currentload _wagondata) (Variables|/Script/LittleRailways.TestWagon|GetcurrentLoad _array_element))
    (Utilities|Array|Add (.spawntransform _wagondata) (Transformation|GetActorTransform _array_element))))

(fn SaveCarriages
  (bind _carriagedata (Variables|Default|GetCarriageData))
  (bind _outactors (Actor|GetAllActorsOfClass "/Script/LittleRailways.CarriageClass"))
  (for _array_element _outactors
    (Utilities|Array|Add (.carriagetypeid _carriagedata) (Variables|/Script/LittleRailways.CarriageClass|GettypeID _array_element))
    (Utilities|Array|Add (.passengercount _carriagedata) (Variables|/Script/LittleRailways.CarriageClass|GetcurrentPassengerCount _array_element))
    (Utilities|Array|Add (.passengerdestinations _carriagedata) (Utilities|Struct|MakeS_PassengerDestinations (Variables|/Script/LittleRailways.CarriageClass|GetpassengerDestinations _array_element)))
    (Utilities|Array|Add (.spawntransform _carriagedata) (Transformation|GetActorTransform _array_element))))

(fn SavePlayerPawn
  (bind _returnvalue (Game|Player|GetPlayerPawn 0))
  ;[1 1 1] If the player is not possessing a train - save player character location to spawn it in
  (Utilities|Casting|CastToLocoController _returnvalue
    (:then
      (Variables|Default|SetisPossessingLoco true))
    (:CastFailed
      (Variables|Default|SetisPossessingLoco false)
      (Variables|Default|SetPlayerCharacterTransform (Transformation|GetActorTransform _returnvalue)))))

(fn SaveProgressionData
  (bind _aslittle_railways_game_mode (Utilities|Casting|CastToLittleRailwaysGameMode (Game|GetGameMode)))
  (Variables|Default|SetProgressionData (Utilities|Struct|MakeS_ProgressionData (Variables|/Script/LittleRailways.LittleRailwaysGameMode|GetcurrentLevel _aslittle_railways_game_mode) (Variables|/Script/LittleRailways.LittleRailwaysGameMode|GetcurrentXP _aslittle_railways_game_mode) (Variables|/Script/LittleRailways.LittleRailwaysGameMode|GetcurrentMoney _aslittle_railways_game_mode))))

(fn SaveData
  ;[1 1 1] Gets all relevant save data and overwrites the data in the current save game object
  (CallFunction|SaveLocos)
  (CallFunction|SaveWagons)
  (CallFunction|SaveCarriages)
  (CallFunction|SavePlayerPawn)
  (CallFunction|SaveProgressionData)
  (Variables|/Game/Blueprints/SaveSystem/BP_SaveGameObject.BP_SaveGameObject_C|SetSaveData (Variables|Default|GetSaveGameObject) (Utilities|Struct|MakeS_SaveData (Variables|Default|GetCarriageData) (Variables|Default|GetWagonData) (Variables|Default|GetLocoData) (Variables|Default|GetProgressionData) (Variables|Default|GetisPossessingLoco) (Variables|Default|GetPlayerCharacterTransform))))

(fn GetHasSaveSlot
  (bind _returnvalue (SaveGame|DoesSaveGameExist "Test"))
  (return _returnvalue))