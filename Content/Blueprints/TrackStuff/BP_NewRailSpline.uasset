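; Spline-driven rail track actor that builds rails and sleepers along its spline in the construction script.
; The spline is split into fixed-length sections, optionally sized by actor X scale, with a flag adding one extra end section.
; Each section gets a spline mesh rail with length-clamped tangents and configurable collision on a custom object channel.
; An instanced static mesh sleeper sits at each section start, aligned with the section.
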(fn ConstructionScript
  (if (Variables|Default|GetAllowScaling)
    (Variables|Default|SetSectionLengthRail (* (.x (Transformation|GetActorScale3D)) 1e+02)))
  (if (Variables|Default|GetMustBeMaxLength)
    (bind _truncatedlength (CallFunction|TruncateSplineLength))
    (for _index (range 0 _truncatedlength)
      (Variables|Default|SetLoopIndex _index)
      (CallFunction|SetRails)
      (CallFunction|SetSleepers))
    (else
      (bind _truncatedlength_2 (CallFunction|TruncateSplineLength))
      (for _index_2 (range 0 (- _truncatedlength_2 1))
        (Variables|Default|SetLoopIndex _index_2)
        (CallFunction|SetRails)
        (CallFunction|SetSleepers)))))

(fn TruncateSplineLength
  (return (Math|Float|Truncate (/ (Spline|GetSplineLength (Variables|Default|GetSpline)) (Variables|Default|GetSectionLengthRail)))))

(fn GetStartPos/Tangents
  (params (LoopIndex :type Integer))
  (bind _sectionlengthrail (Variables|Default|GetSectionLengthRail))
  (bind _spline (Variables|Default|GetSpline))
  (bind _returnvalue (* LoopIndex _sectionlengthrail))
  (return (Spline|GetLocationatDistanceAlongSpline _spline _returnvalue "Local") (Math|Vector|ClampVectorSize (Spline|GetTangentatDistanceAlongSpline _spline _returnvalue "Local") 0.0 (Variables|Default|GetSectionLengthRail))))

(fn GetEndPos/Tangents
  (params (LoopIndex :type Integer))
  (bind _returnvalue (+ LoopIndex 1))
  (bind _sectionlengthrail (Variables|Default|GetSectionLengthRail))
  (bind _spline (Variables|Default|GetSpline))
  (bind _returnvalue_2 (* _returnvalue _sectionlengthrail))
  (return (Spline|GetLocationatDistanceAlongSpline _spline _returnvalue_2 "Local") (Math|Vector|ClampVectorSize (Spline|GetTangentatDistanceAlongSpline _spline _returnvalue_2 "Local") 0.0 (Variables|Default|GetSectionLengthRail))))

(fn SetRails
  (bind _returnvalue (AddComponent|AddSplineMeshComponent false))
  (Components|StaticMesh|SetStaticMesh _returnvalue (Variables|Default|GetSplineMesh))
  (SplineMesh|SetForwardAxis _returnvalue "X" true)
  (bind (_pos _tangent) (CallFunction|GetStartPos/Tangents (Variables|Default|GetLoopIndex)))
  (bind (_pos_2 _tangent_2) (CallFunction|GetEndPos/Tangents (Variables|Default|GetLoopIndex)))
  (SplineMesh|SetStartandEnd _returnvalue _pos _tangent _pos_2 _tangent_2 true :!class /Script/Engine.SplineMeshComponent)
  (Collision|SetCollisionEnabled _returnvalue (Variables|Default|GetCollisionType))
  (Collision|SetCollisionObjectType _returnvalue "ECC_GameTraceChannel3"))

(fn SetSleepers
  (bind _pos (CallFunction|GetStartPos/Tangents (Variables|Default|GetLoopIndex)))
  (bind _pos_2 (CallFunction|GetEndPos/Tangents (Variables|Default|GetLoopIndex)))
  (Components|InstancedStaticMesh|AddInstance (Variables|Default|GetInstancedStaticMesh) (Math|Transform|MakeTransform _pos (Math|Rotator|MakeRotfromX (- _pos _pos_2))) false))