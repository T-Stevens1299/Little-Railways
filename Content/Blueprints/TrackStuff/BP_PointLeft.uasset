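; BP_PointLeft is a track piece, by its name a left-hand point, with separate collision components for its straight and curved routes.
; Its construction script puts both components on the GameTraceChannel3 object channel with query and physics collision enabled.
; The DebugOn flag shows or hides both collision components without propagating to their children.
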(fn ConstructionScript
  (Collision|SetCollisionObjectType (Variables|Default|GetCurvedCollision) "ECC_GameTraceChannel3")
  (Collision|SetCollisionEnabled (Variables|Default|GetStraightCollision) "QueryAndPhysics")
  (if (Variables|Default|GetdebugOn)
    (Rendering|SetVisibility (Variables|Default|GetStraightCollision) true false)
    (else
      (Rendering|SetVisibility (Variables|Default|GetStraightCollision) false false))))