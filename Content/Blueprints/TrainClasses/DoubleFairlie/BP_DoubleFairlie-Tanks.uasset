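; Tank section of the Double Fairlie locomotive, handling its running sound, W-key whistle and chimney steam effects.
; While the throttle is on, Tick reads wheel rotation from the DriverSet1 bogie child actor to time chuffs.
; Entering set angle windows alternates two chuff sounds and switches the steam particle size and velocity to chuff values.
; Outside those windows, or on ToggleStaticSteam, the steam returns to exhaust values.
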(event EventBeginPlay
  (Audio|Components|Audio|Play (Variables|Default|GetLocoSound) 0.0))

(event EventToggleStaticSteam
  (Effects|Components|ParticleSystem|SetFloatParameter (Variables|Default|GetSteamGenerator) "User.chuff_particle_max_size" (Variables|Default|GetExhaustParticleMaxSize))
  (Effects|Components|ParticleSystem|SetVectorParameter (Variables|Default|GetSteamGenerator) "User.chuff_particle_velocity" (Variables|Default|GetExhaustVelocity)))

(event EventTick
  (params (DeltaSeconds :type Float%20%28single-precision%29))
  (if (Variables|Default|GetthrottleOn)
    (CallFunction|SoundCalculations)))

(event Input|KeyboardEvents|W
  (params (Key :type Key%20Structure :default "None"))
  (:Pressed
    (Audio|PlaySoundatLocation "/Game/Sound/DFWhistle.DFWhistle" (Transformation|GetActorLocation) "0, 0, 0" 1.0 1.0 0.0 0 0 0 0)))

(fn ConstructionScript)

(fn SoundCalculations
  (bind _locochuff1 (Variables|Default|GetLocoChuff1))
  (bind _locochuff2 (Variables|Default|GetLocoChuff2))
  (bind _asbp_dffairlie_bogie_red (Utilities|Casting|CastToBP_DFFairlieBogieRed (Variables|/Script/Engine.ChildActorComponent|GetChildActor (Variables|Default|GetDriverSet1))))
  (bind _wheelrot (Default|GetWheelRot _asbp_dffairlie_bogie_red))
  (LocalVariables|SetCurrentWheelRot _wheelrot)
  (if (>= (Variables|Default|GetCurrentPistonStroke) 2)
    (Variables|Default|SetCurrentPistonStroke 0))
  (if (or (and (< (LocalVariables|GetCurrentWheelRot) 6e+01) (> (LocalVariables|GetCurrentWheelRot) 3e+01)) (and (< (LocalVariables|GetCurrentWheelRot) -3e+01) (> (LocalVariables|GetCurrentWheelRot) -6e+01)))
    (if (Math|Boolean|NORBoolean (LocalVariables|GetCycle1Started) (LocalVariables|GetCycle2Started))
      (Variables|Default|SetCurrentPistonStroke (+ (Variables|Default|GetCurrentPistonStroke) 1))
      (if (== 1 (Variables|Default|GetCurrentPistonStroke))
        (Audio|Components|Audio|Stop _locochuff2)
        (Audio|Components|Audio|Play _locochuff1 0.0)
        (LocalVariables|SetCycle1Started true)
        (LocalVariables|SetCycle2Started false)
        (else
          (Audio|Components|Audio|Stop _locochuff1)
          (Audio|Components|Audio|Play _locochuff2 0.0)
          (LocalVariables|SetCycle1Started false)
          (LocalVariables|SetCycle2Started true)))
      (Effects|Components|ParticleSystem|SetFloatParameter (Variables|Default|GetSteamGenerator) "User.chuff_particle_max_size" (Variables|Default|GetChuffParticleMaxSize))
      (Effects|Components|ParticleSystem|SetVectorParameter (Variables|Default|GetSteamGenerator) "User.chuff_particle_velocity" (Variables|Default|GetChuffVelocity)))
    (else
      (LocalVariables|SetCycle1Started false)
      (LocalVariables|SetCycle2Started false)
      (Effects|Components|ParticleSystem|SetFloatParameter (Variables|Default|GetSteamGenerator) "User.chuff_particle_max_size" (Variables|Default|GetExhaustParticleMaxSize))
      (Effects|Components|ParticleSystem|SetVectorParameter (Variables|Default|GetSteamGenerator) "User.chuff_particle_velocity" (Variables|Default|GetExhaustVelocity)))))