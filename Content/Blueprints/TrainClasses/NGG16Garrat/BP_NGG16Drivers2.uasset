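; Second driving-wheel unit of the NG G16 Garratt locomotive, part of the train classes.
; The Construction Script fills WheelsToDrive with three left and right wheel pairs.
; On BeginPlay it casts its root to a static mesh component and passes it to the Coupling child actor as the vehicle body through SetVehicleBodyMessage.
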(event EventBeginPlay
  (bind _asstatic_mesh_component (Utilities|Casting|CastToStaticMeshComponent (Variables|Transformation|GetRootComponent)))
  (Class|BPICoupling|SetVehicleBody(Message) (Variables|/Script/Engine.ChildActorComponent|GetChildActor (Variables|Default|GetCoupling)) _asstatic_mesh_component))

(fn ConstructionScript
  (Variables|Default|SetwheelsToDrive (Utilities|Array|MakeArray (Variables|Default|GetLeftWheel1) (Variables|Default|GetRightWheel1) (Variables|Default|GetLeftWheel2) (Variables|Default|GetRightWheel2) (Variables|Default|GetLeftWheel3) (Variables|Default|GetRightWheel3))))