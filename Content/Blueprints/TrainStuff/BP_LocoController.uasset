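; BP_LocoController is the player-controlled locomotive, handling exit and whistle input.
; The exit action spawns a player actor at a fixed offset from the locomotive, has the first player controller possess it, then clears all widgets.
; Pressing W plays a test whistle at the locomotive's location.
; Logic to pause or resume the locomotive sound based on velocity is present but never runs.
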(event Input|EnhancedActionEvents|EnhancedInputActionIA_Exit
  (params (ActionValue :type Boolean) (ElapsedSeconds :type Float%20%28double-precision%29) (TriggeredSeconds :type Float%20%28double-precision%29) (InputAction :type Input%20Action%20Object%20Reference :default "/Game/FirstPerson/Input/Actions/IA_Exit.IA_Exit"))
  (bind _returnvalue (Game|SpawnActorfromClass (Variables|Default|GetPlayerToSpawn) (Math|Transform|MakeTransform (+ (Transformation|GetActorLocation) "200.000000,200.000000,0.000000") "0, 0, 0" "1.000000,1.000000,1.000000") "Undefined" "MultiplyWithRoot" 0 0))
  (Pawn|Possess (Game|GetPlayerController 0) _returnvalue)
  (Class|LittleRailwaysCharacter|Possessed _returnvalue)
  (Viewport|RemoveAllWidgets))

(event Input|KeyboardEvents|W
  (params (Key :type Key%20Structure :default "None"))
  (:Pressed
    (Audio|PlaySoundatLocation "/Game/Sound/SmallEnglandWhistleTest.SmallEnglandWhistleTest" (Transformation|GetActorLocation) "0, 0, 0" 1.0 1.0 0.0 0 0 0 0)))

(fn ConstructionScript)