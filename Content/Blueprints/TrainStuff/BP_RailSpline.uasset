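; BP_RailSpline is a spline-driven railway track actor that builds sleepers, rails and ballast along its spline.
; The construction script divides the spline into fixed-length sections, adding an instanced sleeper at each one, oriented along the segment.
; Each section also gets separate rail and ballast spline meshes, using tangents clamped to the section length.
; A toggle switches spline mesh collision on or off, under a custom object channel.
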(fn ConstructionScript
  (bind _sectionlength (Variables|Default|GetsectionLength))
  (bind _spline (Variables|Default|GetSpline))
  (bind _spline_2 (Variables|Default|GetSpline))
  (bind _sectionlength_2 (Variables|Default|GetsectionLength))
  (bind _output_get (Variables|Default|SetNum_Instances (Math|Float|Floor (/ (Spline|GetSplineLength (Variables|Default|GetSpline)) (Variables|Default|GetsectionLength)))))
  (for _index (range 0 _output_get)
    (Variables|Default|SetcurLocation (Spline|GetLocationatDistanceAlongSpline _spline_2 (* _index _sectionlength) "Local"))
    (Variables|Default|SetnextLocation (Spline|GetLocationatDistanceAlongSpline _spline (* (+ _index 1) _sectionlength) "Local"))
    (CallFunction|SetSleeper)
    (Variables|Default|SetcurTangent (Math|Vector|ClampVectorSize (Spline|GetTangentatDistanceAlongSpline _spline_2 (* _index _sectionlength) "Local") 0.0 _sectionlength_2))
    (Variables|Default|SetnextTangent (Math|Vector|ClampVectorSize (Spline|GetTangentatDistanceAlongSpline _spline (* (+ _index 1) _sectionlength) "Local") 0.0 _sectionlength_2))
    (CallFunction|SetRails)
    (CallFunction|SetBallast)))

(fn SetSleeper
  (Components|InstancedStaticMesh|AddInstance (Variables|Default|GetSleeperInstance) (Math|Transform|MakeTransform (Variables|Default|GetcurLocation) (Math|Rotator|MakeRotfromX (- (Variables|Default|GetcurLocation) (Variables|Default|GetnextLocation)))) false))

(fn SetRails
  (bind _returnvalue (AddComponent|AddSplineMeshComponent false))
  (bind _output_get (LocalVariables|SetrailsSplineMesh _returnvalue))
  (SplineMesh|SetForwardAxis _output_get "X" true)
  (SplineMesh|SetStartandEnd (LocalVariables|GetrailsSplineMesh) (Variables|Default|GetcurLocation) (Variables|Default|GetcurTangent) (Variables|Default|GetnextLocation) (Variables|Default|GetnextTangent) true :!class /Script/Engine.SplineMeshComponent)
  (Collision|SetCollisionEnabled (LocalVariables|GetrailsSplineMesh) (select (Variables|Default|GetcollisionToggle) "QueryAndPhysics" "NoCollision"))
  (Collision|SetCollisionObjectType (LocalVariables|GetrailsSplineMesh) "ECC_GameTraceChannel3"))

(fn SetBallast
  (bind _returnvalue (AddComponent|AddSplineMeshComponent false))
  (bind _output_get (Variables|Default|SetBallastSplineMesh _returnvalue))
  (SplineMesh|SetForwardAxis _output_get "X" true)
  (SplineMesh|SetStartandEnd (Variables|Default|GetBallastSplineMesh) (Variables|Default|GetcurLocation) (Variables|Default|GetcurTangent) (Variables|Default|GetnextLocation) (Variables|Default|GetnextTangent) true :!class /Script/Engine.SplineMeshComponent)
  (Collision|SetCollisionEnabled (Variables|Default|GetBallastSplineMesh) (select (Variables|Default|GetcollisionToggle) "QueryAndPhysics" "NoCollision"))
  (Collision|SetCollisionObjectType (Variables|Default|GetBallastSplineMesh) "ECC_GameTraceChannel3"))