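; BP_Coupling is a train coupling actor that physically links two vehicle bodies.
; When enabled, overlapping a "Coupling"-tagged component messages the other coupling, which places a physics constraint midway between them, joins both bodies and derives its linear X limit from the gap.
; ToggleCoupling breaks the constraint on both sides if coupled, otherwise arms or disarms coupling.
; The vehicle body is supplied through an event, and other events show or hide an outline.
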(event OnComponentBeginOverlap(OverlapChecker)
  (params (OverlappedComponent :type Primitive%20Component%20Object%20Reference) (OtherActor :type Actor%20Object%20Reference) (OtherComp :type Primitive%20Component%20Object%20Reference) (OtherBodyIndex :type Integer) (bFromSweep :type Boolean) (SweepResult :type Hit%20Result%20Structure%20%28by%20ref%29))
  (if (Variables|Default|GetcanCouple)
    (if (Variables|Default|GetisCoupled)
      (Development|PrintString "Already Coupled")
      (else
        (bind _output_get (Variables|Default|SetOtherCoupling OtherActor))
        (if (Components|ComponentHasTag OtherComp "Coupling")
          (bind _asbp_coupling (Utilities|Casting|CastToBP_Coupling _output_get))
          (Class|BPICoupling|HookLink3Elsewhere(Message) _output_get 0 (Transformation|GetWorldLocation (Variables|/Script/LittleRailways.Coupling|GetOverlapChecker _asbp_coupling)) (Variables|Default|GetThisVehicleBody))
          (Development|PrintString "CoupleBegin" true true "(R=1.000000,G=0.090198,B=0.000000,A=1.000000)")
          (Variables|Default|SetisCoupled true)
          (Variables|Default|SetcanCouple false)
          (else
            (Development|PrintString "Collider not recognised")))))
    (else
      (Development|PrintString "Cannot Couple"))))

(event EventHookLink3Elsewhere
  (params (OtherHook :type Static%20Mesh%20Component%20Object%20Reference) (Link3TargetPos :type Vector :default "0, 0, 0") (OtherVehicleBody :type Static%20Mesh%20Component%20Object%20Reference))
  (bind _overlapchecker (Variables|Default|GetOverlapChecker))
  (bind _returnvalue (Transformation|GetWorldLocation _overlapchecker))
  (Variables|Default|SetMoveTargetPos Link3TargetPos)
  (Variables|Default|SetOther%20Vehicle%20Body OtherVehicleBody)
  (Transformation|SetWorldLocation (Variables|Default|Getbody_to_body_constraint) (+ (/ (- (Variables|Default|GetMoveTargetPos) _returnvalue) 2.0) _returnvalue) false true)
  (Class|PhysicsConstraintComponent|SetConstrainedComponents (Variables|Default|Getbody_to_body_constraint) (Variables|Default|GetThisVehicleBody) "None" (Variables|Default|GetOther%20Vehicle%20Body) "None")
  (Class|PhysicsConstraintComponent|SetLinearXLimit (Variables|Default|Getbody_to_body_constraint) "LCM_Limited" (/ (- (Variables|Default|GetMaxCouplingDistance) (Math|Vector|Distance(Vector) (Variables|Default|GetMoveTargetPos) (Transformation|GetWorldLocation (Variables|Default|GetOverlapChecker)))) 4.0))
  (Variables|Default|SetisCoupled true)
  (Variables|Default|SetcanCouple false)
  (Development|PrintString "CouplingFinished" true true "(R=0.080921,G=1.000000,B=0.000000,A=1.000000)"))

(event EventSetVehicleBody
  (params (VehicleBody :type Static%20Mesh%20Component%20Object%20Reference))
  (Variables|Default|SetThisVehicleBody VehicleBody))

(event EventShowOutline
  (Rendering|SetVisibility (Variables|Default|GetOutline) true false))

(event EventHideOutline
  (Rendering|SetVisibility (Variables|Default|GetOutline) false false))

(event EventToggleCoupling
  (if (Variables|Default|GetisCoupled)
    (Class|PhysicsConstraintComponent|BreakConstraint (Variables|Default|Getbody_to_body_constraint))
    (Development|PrintString "Coupling Broke")
    (Variables|Default|SetisCoupled false)
    (Variables|Default|SetcanCouple false)
    (bind _asbp_coupling (Utilities|Casting|CastToBP_Coupling (Variables|Default|GetOtherCoupling)))
    (Class|PhysicsConstraintComponent|BreakConstraint (Variables|BP_Coupling_C|Getbody_to_body_constraint _asbp_coupling))
    (Variables|BP_Coupling_C|SetisCoupled _asbp_coupling false)
    (Variables|BP_Coupling_C|SetcanCouple _asbp_coupling false)
    (elif (Variables|Default|GetcanCouple)
      (Variables|Default|SetcanCouple false)
      (Development|PrintString "Coupling Disabled")
      (else
        (Variables|Default|SetcanCouple true)
        (Development|PrintString "Coupling Enabled")))))

(fn ConstructionScript)