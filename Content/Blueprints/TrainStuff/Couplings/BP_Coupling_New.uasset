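; Train coupling actor with a grabbable chain link that hooks onto its own hook or another coupler's.
; Dragging uses a runtime physics handle confined to the coupler's local XZ plane, breaking existing constraints on grab.
; The snap trigger re-hooks its own link or messages an incoming link's coupler to attach here.
; Cross-coupling teleports the link, constrains it to that hook, and joins both vehicle bodies with a distance-based linear limit.
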(event OnComponentBeginOverlap(snap_trigger)
  (params (OverlappedComponent :type Primitive%20Component%20Object%20Reference) (OtherActor :type Actor%20Object%20Reference) (OtherComp :type Primitive%20Component%20Object%20Reference) (OtherBodyIndex :type Integer) (bFromSweep :type Boolean) (SweepResult :type Hit%20Result%20Structure%20%28by%20ref%29))
  (if (Components|ComponentHasTag OtherComp "Coupling")
    (if (== OtherComp (Variables|Default|GetLink3))
      (Utilities|IsValid (Variables|Default|GetGrabHandle)
        (:Is%20Valid
          (Utilities|IsValid (Variables|Default|GetOtherLink)
            (:Is%20Valid
              (Physics|Components|PhysicsHandle|ReleaseComponent (Variables|Default|GetGrabHandle)))
            (:Is%20Not%20Valid
              (Variables|Default|SetMoveTargetPos (Transformation|GetWorldLocation (Variables|Default|Getlocal_link_attach_point)))
              (Physics|Components|PhysicsHandle|ReleaseComponent (Variables|Default|GetGrabHandle))
              (Physics|SetSimulatePhysics (Variables|Default|GetLink3) false)
              (Transformation|SetWorldLocation (Variables|Default|GetLink3) (Variables|Default|GetMoveTargetPos) false true)
              (Physics|SetSimulatePhysics (Variables|Default|GetLink3) true)
              (Class|PhysicsConstraintComponent|SetConstrainedComponents (Variables|Default|Getlink3_hook_pc) (Variables|Default|GetLink3) "None" (Variables|Default|GetHook) "None")
              (Variables|Default|SetLinkAttachedLocally true)
              (Variables|Default|SetLinkAttachedElsewhere false)))))
      (else
        (Variables|Default|SetOtherLink OtherComp)
        (bind _output_get (Variables|Default|SetOtherCoupler OtherActor))
        (Class|BPICoupling|HookLink3Elsewhere(Message) _output_get (Variables|Default|GetHook) (Transformation|GetWorldLocation (Variables|Default|Getother_link_attach_point)) (Variables|Default|GetThis%20Vehicle%20Body))))))

(event OnComponentEndOverlap(snap_trigger)
  (params (OverlappedComponent :type Primitive%20Component%20Object%20Reference) (OtherActor :type Actor%20Object%20Reference) (OtherComp :type Primitive%20Component%20Object%20Reference) (OtherBodyIndex :type Integer))
  (if (Components|ComponentHasTag OtherComp "Coupling")
    (Variables|Default|SetOtherLink 0)
    (if (== OtherComp (Variables|Default|GetLink3))
      (Collision|SetCollisionEnabled (Variables|Default|Getsnap_trigger) "NoCollision"))))

(event EventHookLink3Elsewhere
  (params (OtherHook :type Static%20Mesh%20Component%20Object%20Reference) (Link3TargetPos :type Vector :default "0, 0, 0") (OtherVehicleBody :type Static%20Mesh%20Component%20Object%20Reference))
  (bind _snap_trigger (Variables|Default|Getsnap_trigger))
  (bind _returnvalue (Transformation|GetWorldLocation _snap_trigger))
  (Utilities|IsValid (Variables|Default|GetGrabHandle)
    (:Is%20Valid
      (Variables|Default|SetMoveTargetPos Link3TargetPos)
      (Variables|Default|SetOtherVehicleBody OtherVehicleBody)
      (Physics|Components|PhysicsHandle|ReleaseComponent (Variables|Default|GetGrabHandle))
      (Physics|SetSimulatePhysics (Variables|Default|GetLink3) false)
      (Transformation|SetWorldLocation (Variables|Default|GetLink3) (Variables|Default|GetMoveTargetPos) false true)
      (Physics|SetSimulatePhysics (Variables|Default|GetLink3) true)
      (Class|PhysicsConstraintComponent|SetConstrainedComponents (Variables|Default|Getlink3_hook_pc) (Variables|Default|GetLink3) "None" OtherHook "None")
      (Variables|Default|SetLinkAttachedElsewhere true)
      (Variables|Default|SetLinkAttachedLocally false)
      (Transformation|SetWorldLocation (Variables|Default|Getbody_to_body_constraint) (+ (/ (- (Variables|Default|GetMoveTargetPos) _returnvalue) 2.0) _returnvalue) false true)
      (Class|PhysicsConstraintComponent|SetConstrainedComponents (Variables|Default|Getbody_to_body_constraint) (Variables|Default|GetThis%20Vehicle%20Body) "None" (Variables|Default|GetOtherVehicleBody) "None")
      (Class|PhysicsConstraintComponent|SetLinearXLimit (Variables|Default|Getbody_to_body_constraint) "LCM_Limited" (/ (- (Variables|Default|GetMaxCouplingDistance) (Math|Vector|Distance(Vector) (Variables|Default|GetMoveTargetPos) (Transformation|GetWorldLocation (Variables|Default|Getsnap_trigger)))) 2.0)))))

(event EventShowOutline
  (Rendering|SetVisibility (Variables|Default|GetLink3Outline) true false))

(event EventHideOutline
  (Rendering|SetVisibility (Variables|Default|GetLink3Outline) false false))

(event EventSetInteractingActor
  (params (InteractingActor :type Actor%20Object%20Reference))
  (Variables|Default|SetInteracting%20Actor InteractingActor))

(event EventSetVehicleBody
  (params (VehicleBody :type Static%20Mesh%20Component%20Object%20Reference))
  (Variables|Default|SetThis%20Vehicle%20Body VehicleBody))

(event EventMoveItem
  (bind _self self)
  (bind _returnvalue (Transformation|GetActorTransform _self))
  ;[1 1 1] Move Item
  (bind _grabtargetlocation (Class|BPICharacter|GetGrabTargetLocation(Message) (Variables|Default|GetInteracting%20Actor)))
  (bind _output_get (Variables|Default|SetMoveTargetLocalPos _grabtargetlocation))
  (Variables|Default|SetMoveTargetPos (Math|Transform|TransformLocation _returnvalue (Math|Vector|MakeVector (.x (Math|Transform|InverseTransformLocation _returnvalue _output_get)) 0.0 (.z (Math|Transform|InverseTransformLocation _returnvalue _output_get)))))
  (if (Variables|Default|GetLinkAttachedLocally)
    (Utilities|IsValid (Variables|Default|GetOtherLink)
      (:Is%20Not%20Valid
        _)))
  (Utilities|IsValid (Variables|Default|GetGrabHandle)
    (:Is%20Valid
      _)
    (:Is%20Not%20Valid
      (bind _returnvalue_2 (AddComponent|AddPhysicsHandleComponent))
      (Variables|Default|SetGrabHandle _returnvalue_2)
      (Class|PhysicsHandleComponent|GrabComponentatLocation (Variables|Default|GetGrabHandle) (Variables|Default|GetLink3) "None" (Transformation|GetWorldLocation (Variables|Default|GetLink3)))
      (CallFunction|UnhookLink3)))
  (Physics|Components|PhysicsHandle|SetTargetLocation (Variables|Default|GetGrabHandle) (Variables|Default|GetMoveTargetPos))
  (if (Utilities|Enum|Equal(Enum) (Collision|GetCollisionEnabled (Variables|Default|Getsnap_trigger)) "NoCollision")
    (if (> (Math|Vector|Distance(Vector) (Transformation|GetWorldLocation (Variables|Default|GetLink3)) (Transformation|GetWorldLocation (Variables|Default|Getsnap_trigger))) 1e+01)
      (Collision|SetCollisionEnabled (Variables|Default|Getsnap_trigger) "QueryOnly"))))

(event EventReleaseItem
  (Utilities|IsValid (Variables|Default|GetGrabHandle)
    (:Is%20Valid
      (Physics|Components|PhysicsHandle|ReleaseComponent (Variables|Default|GetGrabHandle))
      (Variables|Default|SetGrabHandle 0))))

(fn ConstructionScript)

(fn UnhookLink3
  (Class|PhysicsConstraintComponent|BreakConstraint (Variables|Default|Getlink3_hook_pc))
  (Class|PhysicsConstraintComponent|BreakConstraint (Variables|Default|Getbody_to_body_constraint))
  (Variables|Default|SetLinkAttachedLocally false)
  (Variables|Default|SetLinkAttachedElsewhere false))

(fn HookLocalLink
  (Development|PrintString "HookLocal")
  (Utilities|IsValid (Variables|Default|GetGrabHandle)
    (:Is%20Valid
      (Utilities|IsValid (Variables|Default|GetOtherLink)
        (:Is%20Valid
          (Physics|Components|PhysicsHandle|ReleaseComponent (Variables|Default|GetGrabHandle)))
        (:Is%20Not%20Valid
          (Variables|Default|SetMoveTargetPos (Transformation|GetWorldLocation (Variables|Default|Getlocal_link_attach_point)))
          (Variables|Default|SetLink3CurrentPos (Transformation|GetWorldLocation (Variables|Default|GetLink3)))
          (Physics|Components|PhysicsHandle|ReleaseComponent (Variables|Default|GetGrabHandle))
          (Physics|SetSimulatePhysics (Variables|Default|GetLink3) false))))))