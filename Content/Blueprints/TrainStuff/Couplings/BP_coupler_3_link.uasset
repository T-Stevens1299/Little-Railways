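; Three-link rail vehicle coupler whose end link a player drags with a physics handle, constrained to the vehicle's centreline.
; A snap trigger hooks the released link onto its own hook, or messages the other coupler to hook onto this one.
; Coupling also adds a direct body-to-body constraint with calculated slack, because link constraints cannot handle the tension.
; Grabbing unhooks both constraints, but a locally hooked link stays put while another link occupies its hook.
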(event OnComponentBeginOverlap(snap_trigger)
  (params (OverlappedComponent :type Primitive%20Component%20Object%20Reference) (OtherActor :type Actor%20Object%20Reference) (OtherComp :type Primitive%20Component%20Object%20Reference) (OtherBodyIndex :type Integer) (bFromSweep :type Boolean) (SweepResult :type Hit%20Result%20Structure%20%28by%20ref%29))
  (if (Components|ComponentHasTag OtherComp "interactable")
    (if (== OtherComp (Variables|Default|Getinteractable_mesh))
      (Utilities|IsValid (Variables|Default|Getgrab_handle)
        (:Is%20Valid
          ;[1 1 1] Cannot hook local link03 if other coupler's link03 is attached
          (Utilities|IsValid (Variables|Default|Getother_link03)
            (:Is%20Valid
              (Physics|Components|PhysicsHandle|ReleaseComponent (Variables|Default|Getgrab_handle)))
            (:Is%20Not%20Valid
              (Variables|Default|Setmove_target_pos (Transformation|GetWorldLocation (Variables|Default|Getlocal_link_attach_point)))
              (Physics|Components|PhysicsHandle|ReleaseComponent (Variables|Default|Getgrab_handle))
              (Physics|SetSimulatePhysics (Variables|Default|Getinteractable_mesh) false)
              (Transformation|SetWorldLocation (Variables|Default|Getinteractable_mesh) (Variables|Default|Getmove_target_pos) false true)
              (Physics|SetSimulatePhysics (Variables|Default|Getinteractable_mesh) true)
              (Class|PhysicsConstraintComponent|SetConstrainedComponents (Variables|Default|Getlink03_hook_constraint) (Variables|Default|Getinteractable_mesh) "None" (Variables|Default|Gethook) "None")
              (Variables|Default|Setlink03_attached_locally true)
              (Variables|Default|Setlink03_attached_elsewhere false)))))
      (else
        ;[1 1 1] hook link from other coupler
        (Variables|Default|Setother_link03 OtherComp)
        (bind _output_get (Variables|Default|Setother_coupler OtherActor))
        (Class|BPIInteract|HookLink03Elsewhere(Message) _output_get (Variables|Default|Gethook) (Transformation|GetWorldLocation (Variables|Default|Getother_link_attach_point)) (Variables|Default|Getthis_vehicle_body))))))

(event OnComponentEndOverlap(snap_trigger)
  (params (OverlappedComponent :type Primitive%20Component%20Object%20Reference) (OtherActor :type Actor%20Object%20Reference) (OtherComp :type Primitive%20Component%20Object%20Reference) (OtherBodyIndex :type Integer))
  (if (Components|ComponentHasTag OtherComp "interactable")
    ;[1 1 1] allow this coupler's interactable mesh to be hooked/unhooked
    (Variables|Default|Setother_link03 0)
    (if (== OtherComp (Variables|Default|Getinteractable_mesh))
      ;[1 1 1] to prevent interactable_mesh snapping back onto hook immediately after being unhooked
      (Collision|SetCollisionEnabled (Variables|Default|Getsnap_trigger) "NoCollision"))))

(event EventBeginPlay
  (|CallParentFunction) ; This node is disabled and will not be called.\nDrag off pins to build functionality.
)

(event Collision|EventActorBeginOverlap
  (params (OtherActor :type Actor%20Object%20Reference))
  (|CallParentFunction OtherActor) ; This node is disabled and will not be called.\nDrag off pins to build functionality.
)

(event EventTick
  (params (DeltaSeconds :type Float%20%28single-precision%29))
  (|CallParentFunction DeltaSeconds) ; This node is disabled and will not be called.\nDrag off pins to build functionality.
)

(event EventMoveItem
  (bind _self self)
  (bind _returnvalue (Transformation|GetActorTransform _self))
  (bind _grab_target_location (Class|BPICharacter|GetGrabTargetLocation(Message) (Variables|Default|Getinteracting_actor)))
  (bind _output_get (Variables|Default|Setmove_target_local_pos _grab_target_location))
  (Variables|Default|Setmove_target_pos (Math|Transform|TransformLocation _returnvalue (Math|Vector|MakeVector (.x (Math|Transform|InverseTransformLocation _returnvalue _output_get)) 0.0 (.z (Math|Transform|InverseTransformLocation _returnvalue _output_get)))))
  (if (Variables|Default|Getlink03_attached_locally)
    ;[1 1 1] This coupler's interactable mesh can only be moved if another coupler isn't attached to this coupler's hook
    (Utilities|IsValid (Variables|Default|Getother_link03)
      (:Is%20Not%20Valid
        _)))
  (Utilities|IsValid (Variables|Default|Getgrab_handle)
    (:Is%20Valid
      _)
    (:Is%20Not%20Valid
      (bind _returnvalue_2 (AddComponent|AddPhysicsHandleComponent))
      (Variables|Default|Setgrab_handle _returnvalue_2)
      (Class|PhysicsHandleComponent|GrabComponentatLocation (Variables|Default|Getgrab_handle) (Variables|Default|Getinteractable_mesh) "None" (Transformation|GetWorldLocation (Variables|Default|Getinteractable_mesh)))
      (CallFunction|UnhookLink03)))
  (Physics|Components|PhysicsHandle|SetTargetLocation (Variables|Default|Getgrab_handle) (Variables|Default|Getmove_target_pos))
  (if (Utilities|Enum|Equal(Enum) (Collision|GetCollisionEnabled (Variables|Default|Getsnap_trigger)) "NoCollision")
    (if (> (Math|Vector|Distance(Vector) (Transformation|GetWorldLocation (Variables|Default|Getinteractable_mesh)) (Transformation|GetWorldLocation (Variables|Default|Getsnap_trigger))) 1e+01)
      (Collision|SetCollisionEnabled (Variables|Default|Getsnap_trigger) "QueryOnly"))))

(event EventReleaseItem
  (Utilities|IsValid (Variables|Default|Getgrab_handle)
    (:Is%20Valid
      (Physics|Components|PhysicsHandle|ReleaseComponent (Variables|Default|Getgrab_handle))
      (Variables|Default|Setgrab_handle 0))))

(event EventSetVehicleBody
  (params (vehicle_body :type Static%20Mesh%20Component%20Object%20Reference))
  (Variables|Default|Setthis_vehicle_body vehicle_body))

(event EventHookLink03Elsewhere
  (params (other%20hook :type Static%20Mesh%20Component%20Object%20Reference) (link03%20target%20pos :type Vector :default "0, 0, 0") (other_vehicle_body :type Static%20Mesh%20Component%20Object%20Reference))
  (bind _snap_trigger (Variables|Default|Getsnap_trigger))
  (bind _returnvalue (Transformation|GetWorldLocation _snap_trigger))
  (Utilities|IsValid (Variables|Default|Getgrab_handle)
    (:Is%20Valid
      (Variables|Default|Setmove_target_pos link03%20target%20pos)
      (Variables|Default|Setother_vehicle_body other_vehicle_body)
      (Physics|Components|PhysicsHandle|ReleaseComponent (Variables|Default|Getgrab_handle))
      (Physics|SetSimulatePhysics (Variables|Default|Getinteractable_mesh) false)
      (Transformation|SetWorldLocation (Variables|Default|Getinteractable_mesh) (Variables|Default|Getmove_target_pos) false true)
      (Physics|SetSimulatePhysics (Variables|Default|Getinteractable_mesh) true)
      (Class|PhysicsConstraintComponent|SetConstrainedComponents (Variables|Default|Getlink03_hook_constraint) (Variables|Default|Getinteractable_mesh) "None" other%20hook "None")
      (Variables|Default|Setlink03_attached_elsewhere true)
      (Variables|Default|Setlink03_attached_locally false)
      ;[1 1 1] set the location of the body_to_body_constraint half way between the bodies to be connected
      (Transformation|SetWorldLocation (Variables|Default|Getbody_to_body_constraint) (+ (/ (- (Variables|Default|Getmove_target_pos) _returnvalue) 2.0) _returnvalue) false true)
      ;[1 1 1] The coupling constraints are not strong enough to handle the tension between the rail vehicles, so a direct connection is made
      (Class|PhysicsConstraintComponent|SetConstrainedComponents (Variables|Default|Getbody_to_body_constraint) (Variables|Default|Getthis_vehicle_body) "None" (Variables|Default|Getother_vehicle_body) "None")
      ;[1 1 1] calculate the slack of this constraint based on this coupler's max coupling distance
      (Class|PhysicsConstraintComponent|SetLinearXLimit (Variables|Default|Getbody_to_body_constraint) "LCM_Limited" (/ (- (Variables|Default|Getmax_coupling_distance) (Math|Vector|Distance(Vector) (Variables|Default|Getmove_target_pos) (Transformation|GetWorldLocation (Variables|Default|Getsnap_trigger)))) 2.0)))))

(event EventSetInteractingActor
  (params (interacting_actor :type Actor%20Object%20Reference))
  (Variables|Default|Setinteracting_actor interacting_actor))

(fn ConstructionScript
  (|CallParentFunction))

(fn UnhookLink03
  (Class|PhysicsConstraintComponent|BreakConstraint (Variables|Default|Getlink03_hook_constraint))
  ;[1 1 1] release the main connection between the rail vehicles
  (Class|PhysicsConstraintComponent|BreakConstraint (Variables|Default|Getbody_to_body_constraint))
  (Variables|Default|Setlink03_attached_locally false)
  (Variables|Default|Setlink03_attached_elsewhere false))

(fn HookLocalLink03
  (Utilities|IsValid (Variables|Default|Getgrab_handle)
    (:Is%20Valid
      ;[1 1 1] Cannot hook local link03 if other coupler's link03 is attached
      (Utilities|IsValid (Variables|Default|Getother_link03)
        (:Is%20Valid
          (Physics|Components|PhysicsHandle|ReleaseComponent (Variables|Default|Getgrab_handle)))
        (:Is%20Not%20Valid
          (Variables|Default|Setmove_target_pos (Transformation|GetWorldLocation (Variables|Default|Getlocal_link_attach_point)))
          (Variables|Default|Setlink03_current_pos (Transformation|GetWorldLocation (Variables|Default|Getinteractable_mesh)))
          (Physics|Components|PhysicsHandle|ReleaseComponent (Variables|Default|Getgrab_handle))
          (Physics|SetSimulatePhysics (Variables|Default|Getinteractable_mesh) false))))))

(fn HookOtherLnk03)