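; BP_interact_item is a skeletal interactable item actor in the train couplings folder, apparently a base for child Blueprints.
; Events show or hide an OutlineMesh as a highlight and store interacting and target actor references.
; MoveItem forwards to MoveThisItem, which is an empty stub, and GetCurrentRotation returns a placeholder zero.
; BeginPlay, overlap, Tick and the construction script do nothing.
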(event EventBeginPlay)

(event Collision|EventActorBeginOverlap
  (params (OtherActor :type Actor%20Object%20Reference)))

(event EventTick
  (params (DeltaSeconds :type Float%20%28single-precision%29)))

(event EventShowOutline
  (Rendering|SetVisibility (Variables|Default|Getoutline_mesh) true false))

(event EventHideOutline
  (Rendering|SetVisibility (Variables|Default|Getoutline_mesh) false false))

(event EventSetTargetActor
  (params (target_actor :type Actor%20Object%20Reference))
  (Variables|Default|Settarget_actor target_actor))

(event EventMoveItem
  (CallFunction|MoveThisItem))

(event EventSetInteractingActor
  (params (interacting_actor :type Actor%20Object%20Reference))
  (Variables|Default|Setinteracting_actor interacting_actor))

(fn ConstructionScript)

(fn MoveThisItem)

(fn GetCurrentRotation
  (return 0.0))